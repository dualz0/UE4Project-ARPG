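; AI character that knocks back and damages living characters it runs into while sprinting.
; Capsule hits, gated by a sprint flag exposed through SetSprint/GetSprint, apply a strong horizontal velocity-change impulse away from itself and subtract health via the victim's attribute component.
; Changes to its own health spawn a damage popup widget attached to it, showing the delta.
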(event OnComponentHit(CapsuleComponent)
  (params (HitComponent :type Primitive%20Component%20Object%20Reference) (OtherActor :type Actor%20Object%20Reference) (OtherComp :type Primitive%20Component%20Object%20Reference) (NormalImpulse :type Vector :default "0, 0, 0") (Hit :type Hit%20Result%20Structure%20%28by%20ref%29))
  (bind _issprint (CallFunction|GetSprint))
  (if _issprint
    (bind _ascharacter_base (Utilities|Casting|CastToCharacterBase OtherActor))
    (bind _returnvalue (Class|AttributeComponent|IsActorAlive (Variables|Default|GetAttributeComp) _ascharacter_base))
    (if _returnvalue
      (Physics|AddImpulse (Variables|/Script/Engine.Character|GetCharacterMovement _ascharacter_base) (* (Math|Vector|Normalize (Math|Vector|MakeVector (.X (Math|Vector|BreakVector (- (Transformation|GetActorLocation _ascharacter_base) (Transformation|GetActorLocation)))) (.Y (Math|Vector|BreakVector (- (Transformation|GetActorLocation _ascharacter_base) (Transformation|GetActorLocation)))) 0.0)) 4e+03) true)
      (bind _returnvalue_2 (Class|AttributeComponent|GetAttributeComp _ascharacter_base))
      (Class|AttributeComponent|ApplyHealthChange _returnvalue_2 self -2e+01))))

(event OnHealthChanged(AttributeComp)
  (params (InstigatorActor :type Actor%20Object%20Reference) (OwningComp :type Attribute%20Component%20Object%20Reference) (NewHealth :type Float%20%28single-precision%29) (Delta :type Float%20%28single-precision%29))
  (bind _returnvalue (UserInterface|CreateWidget "/Game/ARPG/Blueprints/UI/Widget_DamagePopup.Widget_DamagePopup_C" 0 self Delta))
  (UserInterface|Viewport|AddtoViewport _returnvalue 0))

(event EventBeginPlay)

(event Collision|EventActorBeginOverlap
  (params (OtherActor :type Actor%20Object%20Reference)))

(event EventTick
  (params (DeltaSeconds :type Float%20%28single-precision%29)))

(fn ConstructionScript)

(fn SetSprint
  (params (IsSprint :type Boolean))
  (Variables|Default|SetbIsSprint IsSprint))

(fn GetSprint
  (return (Variables|Default|GetbIsSprint)))